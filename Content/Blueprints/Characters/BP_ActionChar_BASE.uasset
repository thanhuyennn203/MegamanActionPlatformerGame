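; Base Blueprint for sprite-based action characters, handling damage, defeat and color flash feedback.
; On BeginPlay it creates a dynamic sprite material and plays a flash after a short delay.
; AnyDamage feeds the BPCVitality component until defeated, then either calls Defeated or triggers a stronger flash.
; TriggerFlash sets the material's flash color and multiplier, which a timeline fades to zero; its play-rate setter is unconnected.
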(event `self.ReceiveBeginPlay`
  (bind _returnvalue (`PrimitiveComponent.CreateDynamicMaterialInstance` (`self.Sprite`) 0 null "None"))
  (set `self.DynamicSpriteMat` _returnvalue)
  (`KismetSystemLibrary.Delay` 0.2)
  (`self.TriggerFlash` 1.0 (struct :`R` 1.0 :`G` 0.046667 :`B` 0.249087 :`A` 1.0)))

(event `self.ReceiveAnyDamage`
  (params (Damage :type "Float (single-precision)") (DamageType :type "DamageType Object Reference") (InstigatedBy :type "Controller Object Reference") (DamageCauser :type "Actor Object Reference"))
  (if (not (`/Game/Blueprints/Components/BPC_Vitality.IsDefeated` (`self.BPC_Vitality`)))
    (`/Game/Blueprints/Components/BPC_Vitality.ReceiveDamage` (`self.BPC_Vitality`) Damage)
    (if (`/Game/Blueprints/Components/BPC_Vitality.IsDefeated` (`self.BPC_Vitality`))
      (`self.Defeated`)
      (else
        (`self.TriggerFlash` 10.0 (struct :`R` 1.0 :`G` 0.813263 :`B` 0.018441 :`A` 1.0))))))

(event `TriggerFlash`
  (params (FlashMultiplier :type "Float (single-precision)") (FlashColor :type "LinearColor Structure"))
  (`MaterialInstanceDynamic.SetScalarParameterValue` (`self.DynamicSpriteMat`) "FlashMultiplier" FlashMultiplier)
  (`MaterialInstanceDynamic.SetVectorParameterValue` (`self.DynamicSpriteMat`) "FlashColor" FlashColor)
  (bind (_direction _alpha) (`Timeline|FadeSpriteFlash` :!via `PlayFromStart`)
    (:`Update`
      (`MaterialInstanceDynamic.SetScalarParameterValue` (`self.DynamicSpriteMat`) "FlashMultiplier" (`KismetMathLibrary.Lerp` FlashMultiplier 0.0 _alpha)))))

(fn `UserConstructionScript`)